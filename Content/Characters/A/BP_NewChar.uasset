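; BP_NewChar is a player character Blueprint providing basic movement, jumping and mouse look through Enhanced Input actions.
; MOVE applies movement input along control-rotation directions, flattened by zero pitch, while LOOK feeds controller yaw and pitch.
; On BeginPlay it loops over every row of the ItemDT data table and prints each item's Name, apparently as a data test.
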(event Input|EnhancedActionEvents|EnhancedInputActionIA_Move
  (params (ActionValue :type Vector%202D%20Structure) (ElapsedSeconds :type Float%20%28double-precision%29) (TriggeredSeconds :type Float%20%28double-precision%29) (InputAction :type Input%20Action%20Object%20Reference :default "/Game/Input/Actions/IA_Move.IA_Move"))
  ;[0.15 0.15 0.15 0.5] Movement Inpt
  (CallFunction|MOVE (.x ActionValue) (.y ActionValue)))

(event Input|EnhancedActionEvents|EnhancedInputActionIA_Jump
  (params (ActionValue :type Boolean) (ElapsedSeconds :type Float%20%28double-precision%29) (TriggeredSeconds :type Float%20%28double-precision%29) (InputAction :type Input%20Action%20Object%20Reference :default "/Game/Input/Actions/IA_Jump.IA_Jump"))
  ;[0.15 0.15 0.15 0.5] Jump inpt
  (:Started
    (Character|Jump))
  (:Completed
    (Character|StopJumping)))

(event Input|EnhancedActionEvents|EnhancedInputActionIA_MouseLook
  (params (ActionValue :type Vector%202D%20Structure) (ElapsedSeconds :type Float%20%28double-precision%29) (TriggeredSeconds :type Float%20%28double-precision%29) (InputAction :type Input%20Action%20Object%20Reference :default "/Game/Input/Actions/IA_MouseLook.IA_MouseLook"))
  ;[0.15 0.15 0.15 0.5] Mouse Look inpt
  (CallFunction|LOOK (.x ActionValue) (.y ActionValue)))

(event EventBeginPlay
  (bind _itemdt (Variables|Default|GetItemDT))
  (bind _outrownames (DataTable|GetDataTableRowNames _itemdt))
  (for _array_element _outrownames
    (bind _returnvalue (Utilities|GetDataTableRow _itemdt _array_element)
      (:then
        (Development|PrintString (Utilities|String|ToString(Text) (.Name (Utilities|Struct|BreakS_Item _returnvalue))))))))

(fn ConstructionScript)

(fn MOVE
  (params (X_Axis :type Float%20%28double-precision%29) (Y_Axis :type Float%20%28double-precision%29))
  (bind _returnvalue (Pawn|GetControlRotation :!class /Script/Engine.Pawn))
  ;[0.15 0.15 0.15 0.5] L/R
  (Pawn|Input|AddMovementInput (Math|Vector|GetRightVector (Math|Rotator|MakeRotator (.roll _returnvalue) 0.0 (.yaw _returnvalue))) X_Axis false)
  ;[0.15 0.15 0.15 0.5] FWD/BWD
  (Pawn|Input|AddMovementInput (Math|Vector|GetForwardVector (Math|Rotator|MakeRotator 0.0 0.0 (.yaw (Pawn|GetControlRotation :!class /Script/Engine.Pawn)))) Y_Axis false))

(fn LOOK
  (params (X :type Float%20%28double-precision%29) (Y :type Float%20%28double-precision%29))
  ;[0.15 0.15 0.15 0.5] R/L
  (Pawn|Input|AddControllerYawInput X)
  ;[0.15 0.15 0.15 0.5] U/D
  (Pawn|Input|AddControllerPitchInput Y))