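; AC_Bounce is an actor component that makes its owner bounce incoming lasers by spawning a new emitter for each one.
; Laser hit events add, reposition or remove SC_Emitters in a map keyed by incoming laser, using MirrorLocationRotation on the hit.
; New emitters can inherit the incoming color, and intermediate changes refresh all colors.
; Forced activation and deactivation replay hit start or stop across the owning AC_Handler's filtered lasers.
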(event EventBeginPlay
  (bind _returnvalue (Components|GetOwner))
  (bind _returnvalue_2 (Actor|GetComponentbyClass _returnvalue "/Game/Lasers/Blueprints/BuildingBlocks/AC_Handler.AC_Handler_C"))
  (Utilities|IsValid _returnvalue_2
    (:Is%20Valid
      (Variables|Default|SetOwningHandler _returnvalue_2))))

(event EventInterMediateChange
  (params (Modified :type A%20Laser%20Object%20Reference))
  (bind _values (Utilities|Map|Values (Variables|Default|GetEmmiterBounceMap)))
  (for _array_element _values
    (Default|SetLaserColor _array_element)))

(event EventLaserStopHitting
  (params (Input :type A%20Laser%20Object%20Reference))
  (CallFunction|RemoveLaser Input))

(event EventLasertStartHitting
  (params (Input :type A%20Laser%20Object%20Reference) (Hit%20Info :type Hit%20Result%20Structure))
  (Utilities|IsValid Input
    (:Is%20Valid
      (if (not (Utilities|Map|Contains (Variables|Default|GetEmmiterBounceMap) Input))
        (CallFunction|SpawnLaser Input Hit%20Info)))))

(event EventLasertUpdateHitting
  (params (Input :type A%20Laser%20Object%20Reference) (Hit%20Info :type Hit%20Result%20Structure))
  (bind (_location _rotation) (Utilities|MirrorLocationRotation Hit%20Info))
  (bind _emmiterbouncemap (Variables|Default|GetEmmiterBounceMap))
  (bind (_value _returnvalue) (Utilities|Map|Find _emmiterbouncemap Input))
  (if _returnvalue
    (Transformation|SetWorldLocationAndRotation _value _location _rotation false false)))

(event EventForceActivation
  (params (ApplyConditions :type Boolean))
  (for _array_element (Variables|/Game/Lasers/Blueprints/BuildingBlocks/AC_Handler.AC_Handler_C|GetFilteredLasers (Variables|Default|GetOwningHandler))
    (if (.ReturnValue (Default|GetHitbyHandler _array_element (Variables|Default|GetOwningHandler)))
      (CallFunction|LasertStartHitting _array_element (.Value (Default|GetHitbyHandler _array_element (Variables|Default|GetOwningHandler)))))))

(event EventForceDeactivation
  (params (ApplyConditions :type Boolean))
  (for _array_element (Variables|/Game/Lasers/Blueprints/BuildingBlocks/AC_Handler.AC_Handler_C|GetFilteredLasers (Variables|Default|GetOwningHandler))
    (CallFunction|LaserStopHitting _array_element)))

(fn SpawnLaser
  (params (LaserIn :type A%20Laser%20Object%20Reference) (HitInfo :type Hit%20Result%20Structure))
  (bind _returnvalue (Components|GetOwner))
  (bind _returnvalue_2 (Transformation|GetActorTransform _returnvalue))
  (bind (_location _rotation) (Utilities|MirrorLocationRotation HitInfo))
  (Utilities|IsValid LaserIn
    (:Is%20Valid
      (bind _returnvalue_3 (Game|AddComponentbyClass (Components|GetOwner) "/Game/Lasers/Blueprints/BuildingBlocks/SC_Emitter.SC_Emitter_C" false (Math|Transform|MakeTransform (Math|Transform|InverseTransformLocation _returnvalue_2 _location) (Math|Transform|InverseTransformRotation _returnvalue_2 _rotation) "1.000000,1.000000,1.000000")))
      (Utilities|Map|Add (Variables|Default|GetEmmiterBounceMap) LaserIn _returnvalue_3)
      (if (Variables|Default|GetUseBounceColor)
        (Variables|/Game/Lasers/Blueprints/BuildingBlocks/SC_Emitter.SC_Emitter_C|SetOverrideColor _returnvalue_3 (Variables|/Game/Lasers/Blueprints/BuildingBlocks/A_Laser.A_Laser_C|GetColorOverride LaserIn))
        (Variables|/Game/Lasers/Blueprints/BuildingBlocks/SC_Emitter.SC_Emitter_C|SetUseOverride _returnvalue_3 true))
      (Default|SetLaserColor _returnvalue_3)
      (Default|ActivateLaser _returnvalue_3))))

(fn RemoveLaser
  (params (InputPin :type A%20Laser%20Object%20Reference))
  (bind _emmiterbouncemap (Variables|Default|GetEmmiterBounceMap))
  (bind (_value _returnvalue) (Utilities|Map|Find _emmiterbouncemap InputPin))
  (if _returnvalue
    (bind _output_get (LocalVariables|SetL-RemoveItem _value))
    (Default|ForceDeactivation _output_get false)
    (Default|DestroySelf (LocalVariables|GetL-RemoveItem))
    (Utilities|Map|Remove (Variables|Default|GetEmmiterBounceMap) InputPin)))